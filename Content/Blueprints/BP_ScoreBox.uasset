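; BP_ScoreBox is a scoring trigger that awards the player a point when a rat enters its box.
; On overlap it clears the rat's Cangivescore flag so each rat scores once, then increments the first-person character's score and refreshes its text.
; It also decrements the rat spawner's remaining count, and when none are left it calls Spawnrats after a short delay.
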(event OnComponentBeginOverlap(Box)
  (params (OverlappedComponent :type Primitive%20Component%20Object%20Reference) (OtherActor :type Actor%20Object%20Reference) (OtherComp :type Primitive%20Component%20Object%20Reference) (OtherBodyIndex :type Integer) (bFromSweep :type Boolean) (SweepResult :type Hit%20Result%20Structure%20%28by%20ref%29))
  (bind _asbp_rat (Utilities|Casting|CastToBP_Rat OtherActor))
  (if (Variables|/Game/Blueprints/BP_Rat.BP_Rat_C|Getcangivescore _asbp_rat)
    (Variables|/Game/Blueprints/BP_Rat.BP_Rat_C|Setcangivescore _asbp_rat false)
    (bind _returnvalue (Actor|GetActorOfClass "/Game/FirstPerson/Blueprints/BP_FirstPersonCharacter.BP_FirstPersonCharacter_C"))
    (Math|Integer|IncrementInt (Variables|/Game/FirstPerson/Blueprints/BP_FirstPersonCharacter.BP_FirstPersonCharacter_C|GetScore _returnvalue)
      (:%20%20
        (Default|Updatescoretext _returnvalue)
        (bind _returnvalue_2 (Actor|GetActorOfClass "/Game/Blueprints/BP_RatSpawner.BP_RatSpawner_C"))
        (bind _result (Math|Integer|DecrementInt (Variables|/Game/Blueprints/BP_RatSpawner.BP_RatSpawner_C|Getratsleft _returnvalue_2))
          (:%20%20
            (if (<= _result 0)
              (Utilities|FlowControl|Delay 1.0)
              (Default|Spawnrats _returnvalue_2))))))))

(event EventBeginPlay)

(event Collision|EventActorBeginOverlap
  (params (OtherActor :type Actor%20Object%20Reference)))

(event EventTick
  (params (DeltaSeconds :type Float%20%28single-precision%29)))

(fn ConstructionScript)