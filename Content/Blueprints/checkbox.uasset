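; Trigger-box actor that referees rounds of a bowling-style game where thrown cats take out rats.
; A BP_Cat overlap uses up a player throw and locks input during a short delay.
; The round ends when throws run out or the spawner's rats are gone, then throws reset and rats respawn.
; The player's Cringe or HappyGang reaction depends on rats left, as the Strike flag's print branch is disconnected.
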(event OnComponentBeginOverlap(Box)
  (params (OverlappedComponent :type Primitive%20Component%20Object%20Reference) (OtherActor :type Actor%20Object%20Reference) (OtherComp :type Primitive%20Component%20Object%20Reference) (OtherBodyIndex :type Integer) (bFromSweep :type Boolean) (SweepResult :type Hit%20Result%20Structure%20%28by%20ref%29))
  (bind _player (Variables|Default|Getplayer))
  (Utilities|Casting|CastToBP_Cat OtherActor)
  (bind _result (Math|Integer|DecrementInt (Variables|/Game/FirstPerson/Blueprints/BP_FirstPersonCharacter.BP_FirstPersonCharacter_C|GetTurnThrowsLeft _player))
    (:%20%20
      (Variables|/Game/FirstPerson/Blueprints/BP_FirstPersonCharacter.BP_FirstPersonCharacter_C|SetLockInput _player true)
      (Utilities|FlowControl|Delay 2.0)
      (Variables|/Game/FirstPerson/Blueprints/BP_FirstPersonCharacter.BP_FirstPersonCharacter_C|SetLockInput _player false)
      (if (< _result 1)
        (CallFunction|EndRound false)
        (elif (<= (Variables|/Game/Blueprints/BP_RatSpawner.BP_RatSpawner_C|Getratsleft (Variables|Default|Getspawner)) 0)
          (CallFunction|EndRound true))))))

(event Custom|endRound
  (params (strike :type Boolean))
  (CallFunction|AnnouceRound strike)
  (Variables|/Game/FirstPerson/Blueprints/BP_FirstPersonCharacter.BP_FirstPersonCharacter_C|SetTurnThrowsLeft (Variables|Default|Getplayer) 2)
  (Default|Spawnrats (Variables|Default|GetSpawner)))

(event Custom|AnnouceRound
  (params (strike :type Boolean))
  (if (> (Variables|/Game/Blueprints/BP_RatSpawner.BP_RatSpawner_C|Getratsleft (Variables|Default|Getspawner)) 3)
    (Default|Cringe (Variables|Default|GetPlayer))
    (else
      (Default|HappyGang (Variables|Default|GetPlayer)))))

(event EventBeginPlay
  (bind _returnvalue (Actor|GetActorOfClass "/Game/FirstPerson/Blueprints/BP_FirstPersonCharacter.BP_FirstPersonCharacter_C"))
  (Variables|Default|Setplayer _returnvalue)
  (bind _returnvalue_2 (Actor|GetActorOfClass "/Game/Blueprints/BP_RatSpawner.BP_RatSpawner_C"))
  (Variables|Default|Setspawner _returnvalue_2))

(event EventTick
  (params (DeltaSeconds :type Float%20%28single-precision%29)))

(fn ConstructionScript)