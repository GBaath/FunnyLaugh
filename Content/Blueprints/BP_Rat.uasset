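; BP_Rat is a rat actor that reacts to contact with any actor tagged "Cat".
; Overlap and hit events share one tag check, then pass the offset away from the cat into a custom Hit event.
; That event replaces the mesh's physics velocity with a strong downward vector plus the offset and sets a short lifespan so the rat is destroyed.
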(event Custom|Hit
  (params (inforce :type Vector))
  (Physics|SetPhysicsLinearVelocity (Variables|Default|GetStaticMesh) (+ (* (Math|Vector|VectorUp) -2500) inforce) false "None")
  (Actor|SetLifeSpan 5.0))

(event Custom|OnActorHit_Event
  (params (SelfActor :type Actor%20Object%20Reference) (OtherActor :type Actor%20Object%20Reference) (NormalImpulse :type Vector) (Hit :type Hit%20Result%20Structure%20%28by%20ref%29)))

(event EventBeginPlay)

(event Collision|EventActorBeginOverlap
  (params (OtherActor :type Actor%20Object%20Reference))
  (if (Actor|ActorHasTag (stale Collision|EventHit Other) "Cat")
    (CallFunction|Hit (- (Transformation|GetActorLocation) (Transformation|GetActorLocation (stale Collision|EventHit Other))))))

(event Collision|EventHit
  (params (MyComp :type Primitive%20Component%20Object%20Reference) (Other :type Actor%20Object%20Reference) (OtherComp :type Primitive%20Component%20Object%20Reference) (bSelfMoved :type Boolean) (HitLocation :type Vector :default "0, 0, 0") (HitNormal :type Vector :default "0, 0, 0") (NormalImpulse :type Vector :default "0, 0, 0") (Hit :type Hit%20Result%20Structure%20%28by%20ref%29))
  (if (Actor|ActorHasTag Other "Cat")
    (CallFunction|Hit (- (Transformation|GetActorLocation) (Transformation|GetActorLocation Other)))))

(fn ConstructionScript)